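; BP_MovableWall is a wall actor that temporarily rises when hit by a BP_Laser.
; A valid hit clears the Reactivness flag, then latent MoveComponentTo calls raise and lower the Box component with delays between, restoring the flag after a cooldown.
; Both moves feed offsets from the Box's world location and rotation into relative-space targets.
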(event `self.ReceiveHit`
  (params (MyComp :type "PrimitiveComponent Object Reference") (Other :type "Actor Object Reference") (OtherComp :type "PrimitiveComponent Object Reference") (bSelfMoved :type Boolean) (HitLocation :type "Vector Structure") (HitNormal :type "Vector Structure") (NormalImpulse :type "Vector Structure") (Hit :type "HitResult Structure (by ref)"))
  (`KismetSystemLibrary.PrintString` "Hitted")
  (if (== (`GameplayStatics.GetObjectClass` Other) "/Game/ShootingSystem/Laser/BP_Laser.BP_Laser_C")
    (if (`self.Reactivness`)
      (set `self.Reactivness` false)
      (`self.MoveUp`))))

(event `MoveUp`
  (bind _box (`self.Box`))
  (`KismetSystemLibrary.MoveComponentTo` _box (+ (`SceneComponent.K2_GetComponentLocation` _box) (0.0 0.0 300.0)) (`SceneComponent.K2_GetComponentRotation` _box) false false 3.0)
  (`KismetSystemLibrary.Delay` 7.0)
  (`self.MoveDown`))

(event `MoveDown`
  (bind _box (`self.Box`))
  (`KismetSystemLibrary.MoveComponentTo` _box (+ (`SceneComponent.K2_GetComponentLocation` _box) (0.0 0.0 -300.0)) (`SceneComponent.K2_GetComponentRotation` _box) false false 3.0)
  (`KismetSystemLibrary.Delay` 2.0)
  (set `self.Reactivness` true))

(fn `UserConstructionScript`)