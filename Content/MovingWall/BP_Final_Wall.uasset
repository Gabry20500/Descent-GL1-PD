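; BP_Final_Wall is a blockable moving wall that acts as a door for the player.
; UnlockDoor clears the Blocked flag, after which a BP_Player overlap on its Box calls MoveUp.
; MoveUp uses MoveComponentTo to raise the root 200 units over five seconds, keeping its rotation.
; BeginPlay caches a BP_Player reference, which the shown graphs never use.
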(event `self.ReceiveBeginPlay`
  (bind _returnvalue (`GameplayStatics.GetActorOfClass` "/Game/Player/PlayerMovement/Blueprint/BP_Player.BP_Player_C"))
  (set `self.PG_Ref` _returnvalue))

(event `UnlockDoor`
  (set `self.Blocked` false))

(event `self.Box.OnComponentBeginOverlap`
  (params (OverlappedComponent :type "PrimitiveComponent Object Reference") (OtherActor :type "Actor Object Reference") (OtherComp :type "PrimitiveComponent Object Reference") (OtherBodyIndex :type Integer) (bFromSweep :type Boolean) (SweepResult :type "HitResult Structure (by ref)"))
  (if (`self.Blocked`)
    _
    (elif (== (`GameplayStatics.GetObjectClass` OtherActor) "/Game/Player/PlayerMovement/Blueprint/BP_Player.BP_Player_C")
      (`self.MoveUp`))))

(event `MoveUp`
  (bind _defaultsceneroot (`self.DefaultSceneRoot`))
  (`KismetSystemLibrary.MoveComponentTo` _defaultsceneroot (+ (`SceneComponent.K2_GetComponentLocation` _defaultsceneroot) (0.0 0.0 200.0)) (`SceneComponent.K2_GetComponentRotation` _defaultsceneroot) false false 5.0))

(fn `UserConstructionScript`)