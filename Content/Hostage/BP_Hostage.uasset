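; BP_Hostage is a rescuable hostage pickup that the player collects by touching it.
; On overlap with an actor whose class is exactly BP_Player, it finds the first BP_Player in the level and increments that player's hostage count and adds a fixed score bonus.
; The hostage then destroys itself.
; A debug print of the count is left unconnected.
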(event `self.ReceiveActorBeginOverlap`
  (params (OtherActor :type "Actor Object Reference"))
  (if (== (`GameplayStatics.GetObjectClass` OtherActor) "/Game/Player/PlayerMovement/Blueprint/BP_Player.BP_Player_C")
    (bind _outactors (`GameplayStatics.GetAllActorsOfClass` "/Game/Player/PlayerMovement/Blueprint/BP_Player.BP_Player_C"))
    (bind _output (`|GetArrayItem` _outactors))
    (bind _output_get (set `/Game/Player/PlayerMovement/Blueprint/BP_Player.NumHostage` (+ (`/Game/Player/PlayerMovement/Blueprint/BP_Player.NumHostage` _output) 1) _output))
    (set `/Game/Player/PlayerMovement/Blueprint/BP_Player.Score` (+ (`/Game/Player/PlayerMovement/Blueprint/BP_Player.Score` _output) 1000) _output)
    (`self.K2_DestroyActor`)))

(fn `UserConstructionScript`)