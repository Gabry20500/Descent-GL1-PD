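; BP_EnemyProjectile is an enemy projectile actor whose graph decides what happens when it overlaps another actor.
; After a short delay, a chain of exact class checks filters the overlapped actor.
; Drone and Hulk enemy types only trigger a debug print, while Boss, BP_Missile and BP_Laser are ignored.
; Any other overlap destroys the projectile; this graph applies no damage.
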(event `self.ReceiveActorBeginOverlap`
  (params (OtherActor :type "Actor Object Reference"))
  (bind _returnvalue (`GameplayStatics.GetObjectClass` OtherActor))
  (`KismetSystemLibrary.Delay` 0.1)
  (if (== _returnvalue "/Game/AI/Enemy_Drone_1.Enemy_Drone_1_C")
    (`KismetSystemLibrary.PrintString` "Biebteeeee" true true (struct :`G` 1.0 :`B` 0.451202 :`A` 1.0) :!label _label)
    (elif (== _returnvalue "/Game/AI/Enemy_Drone_2.Enemy_Drone_2_C")
      (goto _label)
      (elif (== _returnvalue "/Game/AI/Enemy_Hulk.Enemy_Hulk_C")
        (goto _label)
        (elif (== _returnvalue "/Game/AI/Hulk_Special.Hulk_Special_C")
          (goto _label)
          (elif (== _returnvalue "/Game/AI/Boss.Boss_C")
            _
            (elif (== _returnvalue "/Game/FightSystem/PlayerProjectile/Missile/BP_Missile.BP_Missile_C")
              _
              (elif (not (== _returnvalue "/Game/FightSystem/PlayerProjectile/Laser/BP_Laser.BP_Laser_C"))
                (`self.K2_DestroyActor`)))))))))

(fn `UserConstructionScript`)