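; AI ship actor that wanders while the player ship overlaps it and turns to face the player once that overlap ends.
; Overlap events toggle a Stopped flag and drive the Movement graph, which chains MoveComponentTo hops to random nearby offsets with a short delay.
; While stopped, Tick calls RotateShip to interpolate rotation toward the player ship found on BeginPlay.
; Shooting nodes (delay, projectile spawn) are unconnected and never run.
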(event `self.ReceiveBeginPlay`
  (bind _returnvalue (`GameplayStatics.GetActorOfClass` "/Game/Player/PlayerMovement/Blueprint/BP_PlayerShip.BP_PlayerShip_C"))
  (set `self.PG_Ref` _returnvalue)
  (`KismetSystemLibrary.PrintString` "Setted"))

(event `self.ReceiveActorBeginOverlap`
  (params (OtherActor :type "Actor Object Reference"))
  (bind (_returnvalue_x _returnvalue_y _returnvalue_z) (`KismetMathLibrary.BreakVector` (`self.K2_GetActorLocation`)))
  (bind _returnvalue (`KismetMathLibrary.RandomFloatInRange` -300.0 300.0))
  (if (== OtherActor (`self.PG_Ref`))
    (set `self.Stopped` false)
    (`KismetSystemLibrary.PrintString` "Moving")
    (`KismetSystemLibrary.MoveComponentTo` (`self.DefaultSceneRoot`) (`KismetMathLibrary.MakeVector` (+ _returnvalue_x _returnvalue) (+ _returnvalue_y _returnvalue) (+ _returnvalue_z (`KismetMathLibrary.RandomFloatInRange` -200.0 200.0))) (struct) false false 2.0 true :!label _label)
    (`KismetSystemLibrary.Delay` 0.1)
    (goto _label)))

(event `self.ReceiveActorEndOverlap`
  (params (OtherActor :type "Actor Object Reference"))
  (if (== OtherActor (`self.PG_Ref`))
    (set `self.Stopped` true)
    (`KismetSystemLibrary.PrintString` "Stopped")
    (goto _label :!via `Stop`)))

(event `self.ReceiveTick`
  (params (DeltaSeconds :type "Float (single-precision)"))
  (if (`self.Stopped`)
    (`self.RotateShip`)))

(fn `RotateShip`
  (bind _returnvalue_location (`KismetMathLibrary.BreakTransform` (`self.GetTransform` (`self.PG_Ref`))))
  (`self.K2_SetActorRotation` (`KismetMathLibrary.RInterpTo` (`self.K2_GetActorRotation`) (`KismetMathLibrary.FindLookAtRotation` (`self.K2_GetActorLocation`) _returnvalue_location) 0.2)))

(fn `UserConstructionScript`)