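; BP_EnErgyPowerUp is an energy pickup for the player.
; On overlap with an actor whose class is exactly BP_Player, it fetches the player through GetActorOfClass rather than casting the overlapping actor.
; If Energy is below 200, it adds 30 without clamping and destroys itself; otherwise the pickup stays in the world.
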(event `self.ReceiveActorBeginOverlap`
  (params (OtherActor :type "Actor Object Reference"))
  (if (== (`GameplayStatics.GetObjectClass` OtherActor) "/Game/Player/PlayerMovement/Blueprint/BP_Player.BP_Player_C")
    (bind _returnvalue (`GameplayStatics.GetActorOfClass` "/Game/Player/PlayerMovement/Blueprint/BP_Player.BP_Player_C"))
    (bind _output_get (set `self.Player` _returnvalue))
    (if (not (>= (`/Game/Player/PlayerMovement/Blueprint/BP_Player.Energy` _output_get) 200))
      (set `/Game/Player/PlayerMovement/Blueprint/BP_Player.Energy` (+ (`/Game/Player/PlayerMovement/Blueprint/BP_Player.Energy` (`self.Player`)) 30) (`self.Player`))
      (`self.K2_DestroyActor`))))

(fn `UserConstructionScript`)