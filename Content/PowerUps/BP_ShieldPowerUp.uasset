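; Shield pickup actor that raises the player's Shield when touched.
; It spins in yaw by a fixed step each tick, independent of delta time.
; On overlap with an exact BP_Player class match, it fetches the player via GetActorOfClass instead of using the overlapping actor.
; If Shield is below the cap, it adds a fixed amount without clamping and destroys itself; otherwise it stays.
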(event `self.ReceiveTick`
  (params (DeltaSeconds :type "Float (single-precision)"))
  (`self.K2_AddActorWorldRotation` (struct :`Yaw` 2.0)))

(event `self.ReceiveActorBeginOverlap`
  (params (OtherActor :type "Actor Object Reference"))
  (if (== (`GameplayStatics.GetObjectClass` OtherActor) "/Game/Player/PlayerMovement/Blueprint/BP_Player.BP_Player_C")
    (bind _returnvalue (`GameplayStatics.GetActorOfClass` "/Game/Player/PlayerMovement/Blueprint/BP_Player.BP_Player_C"))
    (bind _output_get (set `self.Player` _returnvalue))
    (if (not (>= (`/Game/Player/PlayerMovement/Blueprint/BP_Player.Shield` _output_get) 200))
      (set `/Game/Player/PlayerMovement/Blueprint/BP_Player.Shield` (+ (`/Game/Player/PlayerMovement/Blueprint/BP_Player.Shield` (`self.Player`)) 25) (`self.Player`))
      (`self.K2_DestroyActor`))))

(fn `UserConstructionScript`)