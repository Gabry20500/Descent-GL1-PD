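; Player-controlled flyer that moves with six degrees of freedom through swept local offsets and rotations, and can hand possession to a minimap actor.
; Laser and missile shots spawn projectile actors, consuming Energy and missile ammo.
; Box overlaps apply enemy hits, though only Pr1 reduces Shield; the others write Shield minus damage into Energy.
; Tick caps both stats and triggers respawn or loss screen, while a key event unlocks the boss wall.
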(event `self.ReceiveBeginPlay`
  ;[1 1 1] BeginPlay
  (bind _returnvalue (`GameplayStatics.GetActorOfClass` "/Game/Player/PlayerMovement/Blueprint/BP_Player_Map.BP_Player_Map_C"))
  (set `self.MinimapPlayer` _returnvalue))

(event `self.ReceiveTick`
  (params (DeltaSeconds :type "Float (single-precision)"))
  ;[1 1 1] Event Tick
  (`|ExecutionSequence`
    (:`then_0`
      (if (> (`self.Shield`) 200)
        (set `self.Shield` 200)
        (elif (<= (`self.Shield`) 0)
          (`self.Death`))))
    (:`then_1`
      (if (> (`self.Energy`) 200)
        (set `self.Energy` 200)))))

(event `InputAxis|IncreseThrottle`
  (params (AxisValue :type "Float (single-precision)"))
  ;[1 1 1] Increse Throttle
  (if (> AxisValue 0.0)
    (`self.K2_AddActorLocalOffset` (`KismetMathLibrary.MakeVector` (* 6.0 AxisValue)) true)
    (else
      (`self.K2_AddActorLocalOffset` (`KismetMathLibrary.MakeVector` (* AxisValue 6.0)) true))))

(event `Death`
  ;[1 1 1] Death and loose condition
  (if (>= (`self.Lifes`) 0)
    (`self.K2_SetActorLocation` (3097.30835 601.649353 2631.22998))
    (`self.K2_SetActorRotation` (struct :`Yaw` 90.0))
    (set `self.Shield` 100)
    (set `self.Lifes` (- (`self.Lifes`) 1))
    (else
      (bind _returnvalue (`|CreateWidget` "/Game/Player/WinLoseCondition/LoseCondition.LoseCondition_C"))
      (`UserWidget.AddToViewport` _returnvalue 0)
      (`self.DisableInput` null))))

(event `InputAxis|Roll`
  (params (AxisValue :type "Float (single-precision)"))
  ;[1 1 1] Roll
  (if (!= AxisValue 0.0)
    (`self.K2_AddActorLocalRotation` (`KismetMathLibrary.MakeRotator` AxisValue))))

(event `GetKey`
  ;[1 1 1] Get Key
  (set `self.keys` 1)
  (bind _returnvalue (`GameplayStatics.GetActorOfClass` "/Game/MovingWall/BP_Boss_Wall.BP_Boss_Wall_C"))
  (`/Game/MovingWall/BP_Boss_Wall.UnlockDoor` _returnvalue)
  (`KismetSystemLibrary.PrintString` "Final door unlocked"))

(event `Key|M`
  (params (Key :type "Key Structure"))
  ;[1 1 1] Map
  (:`Pressed`
    (`Controller.Possess` (`GameplayStatics.GetPlayerController` 0) (`self.MinimapPlayer`))))

(event `InputAxis|Yaw`
  (params (AxisValue :type "Float (single-precision)"))
  ;[1 1 1] Yaw
  (if (!= AxisValue 0.0)
    (`self.K2_AddActorLocalRotation` (`KismetMathLibrary.MakeRotator` 0.0 0.0 AxisValue))))

(event `InputAxis|Pitch`
  (params (AxisValue :type "Float (single-precision)"))
  ;[1 1 1] Pitch
  (if (!= AxisValue 0.0)
    (`self.K2_AddActorLocalRotation` (`KismetMathLibrary.MakeRotator` 0.0 AxisValue))))

(event `InputAxis|MoveLateral`
  (params (AxisValue :type "Float (single-precision)"))
  ;[1 1 1] MoveLateral
  (if (!= AxisValue 0.0)
    (`self.K2_AddActorLocalOffset` (`KismetMathLibrary.MakeVector` 0.0 (* AxisValue (`self.StrafeSpeed`))) true)))

(event `InputAxis|MoveUp`
  (params (AxisValue :type "Float (single-precision)"))
  ;[1 1 1] MoveUpAndDown
  (if (!= AxisValue 0.0)
    (`self.K2_AddActorLocalOffset` (`KismetMathLibrary.MakeVector` 0.0 0.0 (* AxisValue (`self.StrafeSpeed`))) true)))

(event `InputAction|Laser`
  (params (Key :type "Key Structure"))
  ;[1 1 1] Laser Shoot
  (:`Pressed`
    (if (> (`self.Energy`) 0)
      (set `self.Energy` (- (`self.Energy`) 1))
      (`|SpawnActorFromClass` "/Game/FightSystem/PlayerProjectile/Laser/BP_Laser.BP_Laser_C" (`SceneComponent.K2_GetComponentToWorld` (`self.Spawn_projectile`)) "Undefined" "OverrideRootScale" null null)
      (else
        (`KismetSystemLibrary.PrintString` "Out of Energy")))))

(event `InputAction|Missiles`
  (params (Key :type "Key Structure"))
  (bind _missile_ammo (`self.Missile Ammo`))
  ;[1 1 1] Missile Shoot
  (:`Pressed`
    (if (> _missile_ammo 0)
      (set `self.Missile Ammo` (- _missile_ammo 1))
      (`|SpawnActorFromClass` "/Game/FightSystem/PlayerProjectile/Missile/BP_Missile.BP_Missile_C" (`SceneComponent.K2_GetComponentToWorld` (`self.Spawn_projectile`)) "Undefined" "OverrideRootScale" null null)
      (else
        (`KismetSystemLibrary.PrintString` "Out of Missile")))))

(event `self.Box.OnComponentBeginOverlap`
  (params (OverlappedComponent :type "PrimitiveComponent Object Reference") (OtherActor :type "Actor Object Reference") (OtherComp :type "PrimitiveComponent Object Reference") (OtherBodyIndex :type Integer) (bFromSweep :type Boolean) (SweepResult :type "HitResult Structure (by ref)"))
  (bind _returnvalue (`GameplayStatics.GetObjectClass` OtherActor))
  ;[1 1 1] Player Hitted
  (if (== _returnvalue "/Game/FightSystem/EnemyProjectile/Projectile1/BP_Pr1.BP_Pr1_C")
    (`self.PlayerHittedPr1`)
    (elif (== _returnvalue "/Game/FightSystem/EnemyProjectile/Projectile2/BP_Pr2.BP_Pr2_C")
      (`self.PlayerHittedPr2`)
      (elif (== _returnvalue "/Game/FightSystem/EnemyProjectile/Projectile3/BP_Pr3.BP_Pr3_C")
        (`self.Player Hitted Pr 3`)
        (elif (== _returnvalue "/Game/FightSystem/EnemyProjectile/BossProjectile/BP_BossPr.BP_BossPr_C")
          (`self.Player Hitted Boss`))))))

(fn `Player Hitted Boss`
  (bind (_enemy_prdamage_projectile1 _enemy_prdamage_projectile2 _enemy_prdamage_projectile3 _enemy_prdamage_bossdmg) (break `/Game/FightSystem/EnemyProjectile/Enemy_PrDamage` (`self.Enemy_PrDamage`)))
  ;[1 1 1] Set Player Health
  (bind _output_get (set `self.Energy` (- (`self.Shield`) _enemy_prdamage_bossdmg)))
  (if (not (<= _output_get 0))
    (`KismetSystemLibrary.PrintString` (`KismetStringLibrary.Conv_IntToString` _output_get) true true (struct :`R` 1.0 :`B` 0.050688 :`A` 1.0))))

(fn `Player Hitted Pr 3`
  (bind _enemy_prdamage_projectile1 (break `/Game/FightSystem/EnemyProjectile/Enemy_PrDamage` (`self.Enemy_PrDamage`)))
  ;[1 1 1] Set Player Health
  (bind _output_get (set `self.Energy` (- (`self.Shield`) _enemy_prdamage_projectile1)))
  (if (not (<= _output_get 0))
    (`KismetSystemLibrary.PrintString` (`KismetStringLibrary.Conv_IntToString` _output_get) true true (struct :`R` 1.0 :`B` 0.050688 :`A` 1.0))))

(fn `PlayerHittedPr1`
  (bind _enemy_prdamage_projectile1 (break `/Game/FightSystem/EnemyProjectile/Enemy_PrDamage` (`self.Enemy_PrDamage`)))
  ;[1 1 1] Set Player Health
  (bind _output_get (set `self.Shield` (- (`self.Shield`) _enemy_prdamage_projectile1)))
  (if (not (<= _output_get 0))
    (`KismetSystemLibrary.PrintString` (`KismetStringLibrary.Conv_IntToString` _output_get) true true (struct :`R` 1.0 :`B` 0.050688 :`A` 1.0))))

(fn `PlayerHittedPr2`
  (bind _enemy_prdamage_projectile1 (break `/Game/FightSystem/EnemyProjectile/Enemy_PrDamage` (`self.Enemy_PrDamage`)))
  ;[1 1 1] Set Player Health
  (bind _output_get (set `self.Energy` (- (`self.Shield`) _enemy_prdamage_projectile1)))
  (if (not (<= _output_get 0))
    (`KismetSystemLibrary.PrintString` (`KismetStringLibrary.Conv_IntToString` _output_get) true true (struct :`R` 1.0 :`B` 0.050688 :`A` 1.0))))

(fn `UserConstructionScript`)