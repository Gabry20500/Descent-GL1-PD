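; BP_MinimapPlayer is a player-controlled actor, by its name for the minimap, with six-degree-of-freedom flight controls.
; Input axes drive swept local offsets for throttle, lateral and vertical movement, plus local rotations for roll, yaw and pitch.
; Pressing M stores its ID in MyGameInstance and opens Level1.
; The PlayerHitted functions for projectiles and the boss are empty, with leftover health logic left disconnected.
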(event `InputAxis|IncreseThrottle`
  (params (AxisValue :type "Float (single-precision)"))
  ;[1 1 1] Increse Throttle
  (if (> AxisValue 0.0)
    (`self.K2_AddActorLocalOffset` (`KismetMathLibrary.MakeVector` (* 6.0 AxisValue)) true)
    (else
      (`self.K2_AddActorLocalOffset` (`KismetMathLibrary.MakeVector` (* AxisValue 6.0)) true))))

(event `InputAxis|Roll`
  (params (AxisValue :type "Float (single-precision)"))
  ;[1 1 1] Roll
  (if (!= AxisValue 0.0)
    (`self.K2_AddActorLocalRotation` (`KismetMathLibrary.MakeRotator` AxisValue))))

(event `InputAxis|Yaw`
  (params (AxisValue :type "Float (single-precision)"))
  ;[1 1 1] Yaw
  (if (!= AxisValue 0.0)
    (`self.K2_AddActorLocalRotation` (`KismetMathLibrary.MakeRotator` 0.0 0.0 AxisValue))))

(event `InputAxis|Pitch`
  (params (AxisValue :type "Float (single-precision)"))
  ;[1 1 1] Pitch
  (if (!= AxisValue 0.0)
    (`self.K2_AddActorLocalRotation` (`KismetMathLibrary.MakeRotator` 0.0 AxisValue))))

(event `InputAxis|MoveLateral`
  (params (AxisValue :type "Float (single-precision)"))
  ;[1 1 1] MoveLateral
  (if (!= AxisValue 0.0)
    (`self.K2_AddActorLocalOffset` (`KismetMathLibrary.MakeVector` 0.0 (* AxisValue (`self.StrafeSpeed`))) true)))

(event `InputAxis|MoveUp`
  (params (AxisValue :type "Float (single-precision)"))
  ;[1 1 1] MoveUpAndDown
  (if (!= AxisValue 0.0)
    (`self.K2_AddActorLocalOffset` (`KismetMathLibrary.MakeVector` 0.0 0.0 (* AxisValue (`self.StrafeSpeed`))) true)))

(event `Key|M`
  (params (Key :type "Key Structure"))
  (:`Pressed`
    (bind _asmy_game_instance (cast `/Game/Minimap/MyGameInstance` (`GameplayStatics.GetGameInstance`)))
    (set `/Game/Minimap/MyGameInstance.ID` (`self.ID`) _asmy_game_instance)
    (`GameplayStatics.OpenLevel` "Level1")))

(fn `Player Hitted Boss`
  ;[1 1 1] Set Player Health
)

(fn `Player Hitted Pr 3`
  ;[1 1 1] Set Player Health
)

(fn `PlayerHittedPr1`
  ;[1 1 1] Set Player Health
)

(fn `PlayerHittedPr2`
  ;[1 1 1] Set Player Health
)

(fn `UserConstructionScript`)