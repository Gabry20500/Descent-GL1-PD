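; Player-controlled ship pawn with six-axis style flight (throttle, yaw, pitch, strafing) and laser fire.
; Throttle input sets DesiredSpeed through W/S helper functions, and Tick interpolates CurrentSpeed toward it to move the ship along its local forward axis.
; Rotation and strafing apply local offsets directly, with translations swept and cube hits zeroing CurrentSpeed.
; The Laser action spawns Laser_BP at the SpawnProjectile transform.
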(event `self.ReceiveTick`
  (params (DeltaSeconds :type "Float (single-precision)"))
  ;[1 1 1] On Tick move foreward/backward
  (bind _output_get (set `self.CurrentSpeed` (`KismetMathLibrary.FInterpTo` (`self.CurrentSpeed`) (`self.DesiredSpeed`) (`GameplayStatics.GetWorldDeltaSeconds`) (/ (`self.AcceleratrionInterp`) 2.0))))
  (`self.K2_AddActorLocalOffset` (`KismetMathLibrary.MakeVector` _output_get) true))

(event `InputAxis|IncreseThrottle`
  (params (AxisValue :type "Float (single-precision)"))
  ;[1 1 1] Throttle
  (if (> AxisValue 0.0)
    (set `self.DesiredSpeed` (`KismetMathLibrary.FInterpTo` (`self.DesiredSpeed`) (`self.MaxSpeed`) (`GameplayStatics.GetWorldDeltaSeconds`) (`self.AcceleratrionInterp`)))
    (elif (< AxisValue 0.0)
      (set `self.DesiredSpeed` (`KismetMathLibrary.FInterpTo` (`self.DesiredSpeed`) (* (/ (`self.MaxSpeed`) 2.0) -1.0) (`GameplayStatics.GetWorldDeltaSeconds`) (`self.AcceleratrionInterp`))))))

(event `InputAxis|Yaw`
  (params (AxisValue :type "Float (single-precision)"))
  (if (!= AxisValue 0.0)
    (`self.K2_AddActorLocalRotation` (`KismetMathLibrary.MakeRotator` 0.0 0.0 AxisValue))))

(event `InputAxis|Pitch`
  (params (AxisValue :type "Float (single-precision)"))
  (if (!= AxisValue 0.0)
    (`self.K2_AddActorLocalRotation` (`KismetMathLibrary.MakeRotator` 0.0 AxisValue))))

(event `InputAxis|MoveLateral`
  (params (AxisValue :type "Float (single-precision)"))
  ;[1 1 1] Strafing
  (if (!= AxisValue 0.0)
    (`self.K2_AddActorLocalOffset` (`KismetMathLibrary.MakeVector` 0.0 (* AxisValue (`self.StrafeSpeed`))) true)))

(event `InputAxis|MoveUp`
  (params (AxisValue :type "Float (single-precision)"))
  ;[1 1 1] Strafing
  (if (!= AxisValue 0.0)
    (`self.K2_AddActorLocalOffset` (`KismetMathLibrary.MakeVector` 0.0 0.0 (* AxisValue (`self.StrafeSpeed`))) true)))

(event `self.Cube.OnComponentHit`
  (params (HitComponent :type "PrimitiveComponent Object Reference") (OtherActor :type "Actor Object Reference") (OtherComp :type "PrimitiveComponent Object Reference") (NormalImpulse :type "Vector Structure") (Hit :type "HitResult Structure (by ref)"))
  (set `self.CurrentSpeed` 0.0))

(event `InputAction|Laser`
  (params (Key :type "Key Structure"))
  (:`Pressed`
    (`|SpawnActorFromClass` "/Game/ShootingSystem/Laser/Laser_BP.Laser_BP_C" (`SceneComponent.K2_GetComponentToWorld` (`self.Spawn_projectile`)) "Undefined" "OverrideRootScale" null null)))

(fn `UserConstructionScript`)